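; Test Blueprint that exercises custom shader and compute shader calls on the shared render target RT_ShaderTest.
; BeginPlay clears the target and draws the test shader with the Lion texture; keys 1-4 change color settings and redraw.
; Key 5 enables a per-tick compute shader pass with a cycling red value.
; Key 6 stops that pass and has every VolumetricClouds actor render once into the target.
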(event `self.ReceiveBeginPlay`
  (`KismetRenderingLibrary.ClearRenderTarget2D` "/Game/Blueprint/RT_ShaderTest.RT_ShaderTest")
  (`TestShaderBlueprintLibrary.DrawTestShaderRenderTarget` "/Game/Blueprint/RT_ShaderTest.RT_ShaderTest" self (`self.MyColor`) "/Game/Blueprint/lion.lion" (make `MyShaderStructData` (struct :`R` 1.0 :`G` 0.816467 :`B` 0.040648) (struct :`G` 1.0 :`B` 0.686669) (struct :`R` 0.974842 :`G` 0.016521 :`B` 1.0) (struct :`R` 0.978041 :`G` 0.976708 :`B` 1.0) (`self.ColorIndex`)) :!label _label))

(event `Key|One`
  (params (Key :type "Key Structure"))
  (:`Pressed`
    (set `self.MyColor` (struct :`R` 1.0 :`G` 0.082433 :`A` 1.0))
    (set `self.ColorIndex` 0)
    (set `self.UseCS` false :!label _label_2)
    (set `self.UseCS2` false)
    (goto _label)))

(event `Key|Two`
  (params (Key :type "Key Structure"))
  (:`Pressed`
    (set `self.MyColor` (struct :`R` 0.215702 :`G` 0.989583 :`B` 0.13134 :`A` 1.0))
    (set `self.ColorIndex` 1)
    (goto _label_2)))

(event `Key|Three`
  (params (Key :type "Key Structure"))
  (:`Pressed`
    (set `self.MyColor` (struct :`R` 0.052869 :`B` 1.0 :`A` 1.0))
    (set `self.ColorIndex` 2)
    (goto _label_2)))

(event `Key|Four`
  (params (Key :type "Key Structure"))
  (:`Pressed`
    (set `self.ColorIndex` 3)
    (goto _label_2)))

(event `Key|Five`
  (params (Key :type "Key Structure"))
  (:`Pressed`
    (set `self.UseCS` true)
    (set `self.UseCS2` false)))

(event `Key|Six`
  (params (Key :type "Key Structure"))
  (:`Pressed`
    (set `self.UseCS2` true)
    (set `self.UseCS` false)
    (bind _outactors (`GameplayStatics.GetAllActorsOfClass` "/Script/ShadertestPlugin.VolumetricClouds"))
    (for _array_element _outactors
      (`VolumetricClouds.RenderCloud` _array_element "/Game/Blueprint/RT_ShaderTest.RT_ShaderTest"))))

(event `self.ReceiveTick`
  (params (DeltaSeconds :type "Float (single-precision)"))
  (if (`self.UseCS`)
    (bind _output_get (set `self.DynamicR` (+ (`self.DynamicR`) 0.01)))
    (`TestShaderBlueprintLibrary.UseMyComputeShader` "/Game/Blueprint/RT_ShaderTest.RT_ShaderTest" self (make `MyShaderStructData` (make `LinearColor` (`self.DynamicR`) 0.062383 0.0 1.0) (struct) (struct) (`self.ColorFour`)))
    (if (>= _output_get 10.0)
      (set `self.DynamicR` 0.0))))

(fn `UserConstructionScript`)