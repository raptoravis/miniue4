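; Test actor that draws a custom shader into the RT_ShaderTest render target using a color and the Lion texture.
; BeginPlay clears the target to a fixed color, then calls DrawTestShaderRenderTarget.
; Keys 1, 2 and 3 set Color to an orange-red, green or blue and redraw through the same call without clearing again.
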(event `self.ReceiveBeginPlay`
  (`KismetRenderingLibrary.ClearRenderTarget2D` "/Game/Blueprint/RT_ShaderTest.RT_ShaderTest" (struct :`R` 0.989583 :`G` 0.295795 :`B` 0.087045 :`A` 1.0))
  (`SimplePixelShaderBlueprintLibrary.DrawTestShaderRenderTarget` "/Game/Blueprint/RT_ShaderTest.RT_ShaderTest" (`self.Color`) "/Game/Blueprint/lion.lion" :!label _label))

(event `Key|One`
  (params (Key :type "Key Structure"))
  (:`Pressed`
    (set `self.Color` (struct :`R` 0.994792 :`G` 0.136398 :`A` 1.0))
    (goto _label)))

(event `Key|Two`
  (params (Key :type "Key Structure"))
  (:`Pressed`
    (set `self.Color` (struct :`R` 0.114653 :`G` 1.0 :`A` 1.0))
    (goto _label)))

(event `Key|Three`
  (params (Key :type "Key Structure"))
  (:`Pressed`
    (set `self.Color` (struct :`G` 0.083936 :`B` 1.0 :`A` 1.0))
    (goto _label)))

(fn `UserConstructionScript`)